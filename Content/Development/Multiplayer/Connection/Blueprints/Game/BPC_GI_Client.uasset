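; Client-side multiplayer connection component that logs into PlayFab with a generated custom ID and handles matchmaking to dedicated servers.
; It connects to a hardcoded WebSocket server, sends a VaRest-built JSON findingmatch request with a fixed Elo, and parses the replies.
; A servermatch reply supplies the host and port, which the client joins through an open console command.
; Local games skip matchmaking and open the stored address directly.
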(event Custom|WebSocketConnected
  (params (bWasSuccess :type Boolean) (Response :type String))
  ;[0 0 0] WebSocket Handler And Connection
  (Variables|Default|SetIsConnectedToServer bWasSuccess))

(event Custom|OnWebSocketMessageReceived
  (params (bWasSuccess :type Boolean) (Response :type String))
  ;[0 0 0] WebSocket Handler And Connection
  (CallFunction|WebSocketMessageParse Response))

(event Custom|OnFailurePlayFabLogin
  (params (error :type Play%20Fab%20Error%20Structure) (customData :type Object%20Object%20Reference))
  (bind (_haserror _errorcode _errorname _errormessage _errordetails) (Utilities|Struct|BreakPlayFabError error))
  ;[0 0 0] Failure Play Fab Login Handle
  (Development|PrintString _errorname true true "(R=0.000000,G=0.660000,B=1.000000,A=1.000000)" 2e+02)
  (Development|PrintString _errormessage true true "(R=0.000000,G=0.660000,B=1.000000,A=1.000000)" 2e+02)
  (Development|PrintString _errordetails true true "(R=0.000000,G=0.660000,B=1.000000,A=1.000000)" 2e+02))

(event Custom|WebSocketMessageParse
  (params (Response :type String))
  ;[0 0 0] WebSocket Connected To Server
  (bind _returnvalue (Class|VaRestSubsystem|DecodeJsonObject (|VaRestSubsystem) Response))
  (Utilities|IsValid _returnvalue
    (:Is%20Valid
      (if (Utilities|Enum|Equal(Enum) (Class|VaRestJsonObject|GetStringField _returnvalue "type") "connection_success")
        (Variables|Default|SetIsConnectedToServer true)
        (Development|PrintString "CONNECTED TO SERVER" true true "(R=0.000000,G=0.660000,B=1.000000,A=1.000000)" 2e+01)
        (elif (Utilities|Enum|Equal(Enum) (Class|VaRestJsonObject|GetStringField _returnvalue "type") "servermatch")
          (Variables|Default|SetHostToConnect (Class|VaRestJsonObject|GetStringField (Class|VaRestJsonObject|GetObjectField _returnvalue "data") "host"))
          (Variables|Default|SetPortToConnect (Class|VaRestJsonObject|GetStringField (Class|VaRestJsonObject|GetObjectField _returnvalue "data") "port"))
          (CallFunction|ConnecttoDedicatedServerInstance))))))

(event Custom|SendSearchMatchMessageToServer
  ;[0 0 0] Send Message To Find
  (if (Variables|Default|GetIsLocalGame)
    (CallFunction|ConnecttoDedicatedServerInstance)
    (else
      (bind _returnvalue (Class|VaRestSubsystem|ConstructVaRestJsonObject (|VaRestSubsystem)))
      (Class|VaRestJsonObject|SetStringField _returnvalue "type" "findingmatch")
      (bind _returnvalue_2 (Class|VaRestSubsystem|ConstructVaRestJsonObject (|VaRestSubsystem)))
      (Class|VaRestJsonObject|SetStringField _returnvalue_2 "elo" "100")
      (Class|VaRestJsonObject|SetObjectField _returnvalue "data" _returnvalue_2)
      (Class|WebsocketSubsystem|SendWebSocketMessage (Subsystems|GetWebsocketSubsystem) (Class|VaRestJsonObject|EncodeJsontoSingleString _returnvalue))
      (Development|PrintString "CALLING TO SEARCH MATCH" true true "(R=0.000000,G=0.660000,B=1.000000,A=1.000000)" 2e+01))))

(event Custom|ConnectToDedicatedServerInstance
  (Development|ExecuteConsoleCommand (Utilities|String|Append "open " (Variables|Default|GetHostToConnect) ":" (Variables|Default|GetPortToConnect)) 0))

(event Custom|OnSuccessLoginWithSteam
  (params (result :type Client%20Login%20Result%20Structure) (customData :type Object%20Object%20Reference))
  (bind (_entitytoken _inforesultpayload _lastlogintime _newlycreated _playfabid) (Utilities|Struct|BreakClientLoginResult result))
  ;[0 0 0] Login to Playfab
  (Variables|Default|SetEntityToken _entitytoken)
  (Variables|Default|SetPlay%20Fab%20Id _playfabid))

(event Custom|LoginToPlayFab
  ;[0 0 0] Login to Playfab
  (bind _returnvalue (Class|UtilsGameInstance|GenerateCustomID))
  (bind _successful (|LoginwithCustomID (Utilities|Struct|MakeClientLoginWithCustomIDRequest true _returnvalue) (delegate Custom|OnSuccessLoginWithSteam) (EventDispatchers|CreateEvent :!event Custom|OnFailurePlayFabLogin))
    (:OnPlayFabResponse
      (Variables|Default|SetIsConnectedToPlayFab _successful))))

(event EventConnecttoServer
  (params (Player%20ID :type String))
  (bind _returnvalue (Subsystems|GetWebsocketSubsystem))
  ;[0 0 0] WebSocket Handler And Connection
  (Utilities|IsValid _returnvalue
    (:Is%20Valid
      (EventDispatchers|BindEventtoResponseonConnected _returnvalue (delegate Custom|WebSocketConnected))
      (EventDispatchers|BindEventtoResponseonMessage _returnvalue (delegate Custom|OnWebSocketMessageReceived))
      (Class|WebsocketSubsystem|ConnectWebSocket _returnvalue "ws://3.140.128.226:4000"))))

(event EventInit
  ;[0 0 0] Start
  (Class|PlayFabUtilities|SetPlayFabSettings (Variables|Default|GetGame%20Title%20Id) (Variables|Default|GetPlay%20Fab%20Secret%20Api%20Key)))

(fn GetMatchMakingServer
  (params (Response :type String))
  (bind _returnvalue (Class|VaRestSubsystem|DecodeJsonObject (|VaRestSubsystem) Response))
  (Utilities|IsValid _returnvalue
    (:Is%20Valid
      (if (Utilities|Enum|Equal(Enum) (Class|VaRestJsonObject|GetStringField _returnvalue "type") "servermatch")
        (bind _returnvalue_2 (Class|VaRestJsonValue|AsObject (Class|VaRestJsonObject|GetField _returnvalue "data")))
        (Development|ExecuteConsoleCommand (Utilities|String|Append "open " (Class|VaRestJsonObject|GetFieldTypeString _returnvalue_2 "host") ":" (Class|VaRestJsonObject|GetFieldTypeString _returnvalue_2 "port")) 0)
        (return)))))