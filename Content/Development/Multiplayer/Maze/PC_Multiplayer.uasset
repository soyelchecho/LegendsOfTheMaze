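; Player controller for the multiplayer maze mode that handles player spawning and HUD input.
; On BeginPlay, the local controller requests a server spawn, which GM_Multiplayer performs and returns as PlayerRef, then caches the HUD base.
; Render_HealthBar has the HUD create a health bar menu for that player.
; The P key requests another spawn, while I and M toggle the HUD's inventory and sample menu.
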(event Custom|Server_SpawnPlayer
  (bind _asgm_multiplayer (Utilities|Casting|CastToGM_Multiplayer (Game|GetGameMode)))
  (bind _playerspawned (Default|SpawnPlayer _asgm_multiplayer self))
  (Variables|Default|SetPlayerRef _playerspawned))

(event Custom|Render_HealthBar
  (Default|CreateHealthBarMenu (Variables|Default|GetAs%20HUD%20Base) (Variables|Default|GetPlayerRef)))

(event EventBeginPlay
  (if (Pawn|IsLocalPlayerController)
    (CallFunction|ServerSpawnPlayer)
    (bind _ashud_base (Utilities|GetHUDBase 0.0)
      (:Success
        (Variables|Default|SetAs%20HUD%20Base _ashud_base)))))

(event Input|KeyboardEvents|P
  (params (Key :type Key%20Structure))
  (:Pressed
    (CallFunction|ServerSpawnPlayer)))

(event Input|KeyboardEvents|M
  (params (Key :type Key%20Structure))
  (:Released
    (Default|ToggleSampleMenu (Variables|Default|GetAs%20HUD%20Base))))

(event Input|KeyboardEvents|I
  (params (Key :type Key%20Structure))
  (:Released
    (Default|ToggleInventory (Variables|Default|GetAs%20HUD%20Base))))

(fn ConstructionScript)