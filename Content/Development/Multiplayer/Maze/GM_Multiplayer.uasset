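; Game mode for the multiplayer Maze that tracks connected player controllers and provides player spawning.
; PostLogin and OnSwapPlayerControllers add controllers to AllConnectedPlayers, while OnLogout removes exiting PC_Multiplayer controllers; a swap does not remove the old one.
; SpawnPlayer, not called within this graph, destroys any existing pawn, then spawns and possesses a BP_MultiplayerCharacter at a random PlayerStart.
; BeginPlay only prints a dedicated server start message.
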(event EventBeginPlay
  (Development|PrintString "START DEDICATED SERVER" true true "(R=0.000000,G=0.660000,B=1.000000,A=1.000000)" 2e+01))

(event EventTick
  (params (DeltaSeconds :type Float%20%28single-precision%29)))

(event EventPostLogin
  (params (NewPlayer :type Player%20Controller%20Object%20Reference))
  (Utilities|Array|Add (Variables|Default|GetAllConnectedPlayers) NewPlayer))

(event EventOnSwapPlayerControllers
  (params (OldPC :type Player%20Controller%20Object%20Reference) (NewPC :type Player%20Controller%20Object%20Reference))
  (Utilities|Array|Add (Variables|Default|GetAllConnectedPlayers) NewPC))

(event EventOnLogout
  (params (ExitingController :type Controller%20Object%20Reference))
  (bind _aspc_multiplayer (Utilities|Casting|CastToPC_Multiplayer ExitingController))
  (Utilities|Array|RemoveItem (Variables|Default|GetAllConnectedPlayers) _aspc_multiplayer))

(fn ConstructionScript)

(fn FindRandomPlayerStart
  (bind _outactors (Actor|GetAllActorsOfClass "/Script/Engine.PlayerStart"))
  (return (Transformation|GetActorTransform (Utilities|Array|Get(acopy) _outactors (Math|Random|RandomIntegerinRange 0 (- (Utilities|Array|Length _outactors) 1))))))

(fn SpawnPlayer
  (params (PlayerController :type Player%20Controller%20Object%20Reference))
  (bind _returnvalue (Pawn|GetControlledPawn PlayerController))
  (Utilities|IsValid _returnvalue
    (:Is%20Valid
      (Actor|DestroyActor _returnvalue))
    (:Is%20Not%20Valid
      _))
  (bind _returnvalue_2 (Game|SpawnActorfromClass "/Game/Development/Character/BP_MultiplayerCharacter.BP_MultiplayerCharacter_C" (Spawning|FindRandomPlayerStart) "Undefined" 0 0))
  (Pawn|Possess PlayerController _returnvalue_2)
  (return _returnvalue_2))