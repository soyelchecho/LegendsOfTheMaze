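; PW_Login is a Login level Blueprint that starts the PlayFab login as soon as play begins.
; BeginPlay calls a custom event that casts the game instance to BPC_GI_Client and runs its LoginToPlayFab.
; A disconnected chain that would show the UW_Login widget with cursor and Game and UI input before logging in never runs.
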(event Custom|CallLoginToPlayFab
  ;[1 1 1] Call to Login
  (bind _asbpc_gi_client (Utilities|Casting|CastToBPC_GI_Client (Game|GetGameInstance)))
  (Utilities|IsValid _asbpc_gi_client
    (:Is%20Valid
      (Default|LogintoPlayFab _asbpc_gi_client))))

(event EventBeginPlay
  ;[1 1 1] Add Background Widget
  (CallFunction|CallLogintoPlayFab))

(fn ConstructionScript)