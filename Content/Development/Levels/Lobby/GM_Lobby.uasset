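; Lobby Game Mode that keeps trying to connect the client to a server and can create an online session.
; A looping one-second timer from BeginPlay runs ConnectToServer, which calls the BPC_GI_Client game instance whenever it reports no connection.
; The separate RunCreationServer event creates a non-LAN session for the first player controller and prints success or failure, with no caller in this graph.
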(event Custom|RunCreationServer
  (Development|PrintText "Create Ssssion Server" true true "(R=0.000000,G=0.660000,B=1.000000,A=1.000000)" 15.0)
  (|Session (Game|GetPlayerController 0) 5 false
    (:OnSuccess
      (Development|PrintText "Server Creado" true true "(R=0.000000,G=0.660000,B=1.000000,A=1.000000)" 15.0))
    (:OnFailure
      (Development|PrintText "Fallo Creando Server" true true "(R=0.000000,G=0.660000,B=1.000000,A=1.000000)" 15.0))))

(event Custom|TryToConnectServer
  (CallFunction|ConnecttoServer))

(event EventBeginPlay
  (Utilities|Time|SetTimerbyEvent (delegate Custom|TryToConnectServer) 1.0 true))

(event EventTick
  (params (DeltaSeconds :type Float%20%28single-precision%29)))

(fn ConstructionScript)

(fn ConnecttoServer
  (bind _asbpc_gi_client (Utilities|Casting|CastToBPC_GI_Client (Game|GetGameInstance)))
  (Utilities|IsValid _asbpc_gi_client
    (:Is%20Valid
      (if (not (Variables|/Game/Development/Multiplayer/Connection/Blueprints/Game/BPC_GI_Client.BPC_GI_Client_C|GetIsConnectedToServer _asbpc_gi_client))
        (Development|PrintString "Trying to connect to server" true true "(R=0.000000,G=0.660000,B=1.000000,A=1.000000)" 2e+01)
        (Default|ConnecttoServer _asbpc_gi_client)
        (bind _asbpc_gi_client_2 (Utilities|Casting|CastToBPC_GI_Client (Game|GetGameInstance)))
        (Utilities|IsValid _asbpc_gi_client_2
          (:Is%20Valid
            (Variables|Default|SetIsConnectedToServer (Variables|/Game/Development/Multiplayer/Connection/Blueprints/Game/BPC_GI_Client.BPC_GI_Client_C|GetIsConnectedToServer _asbpc_gi_client_2))))))))