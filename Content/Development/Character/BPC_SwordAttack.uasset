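; Actor component that runs a sword combo for BP_MultiplayerCharacter by playing attack montages.
; SwordAttack starts the attack for the current AttackIndex or buffers input while attacking; SwordAttackCombo then continues the chain or resets it.
; Attack1 plays its montage on player character 0, while later attacks use the cached owner mesh.
; Attack3 is unreachable from the match, and RPCAttack1 is an empty stub.
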(event Custom|SwordAttackCombo
  ;[0.051 0.051 0.051] Combo Continue
  (if (Variables|Default|GetsaveAttack)
    (Variables|Default|SetsaveAttack false)
    (switch int (Variables|Default|GetAttackIndex)
      (:0
        (CallFunction|Attack1))
      (:1
        (CallFunction|Attack2)))
    (else
      (CallFunction|StopCombo))))

(event Custom|Attack2
  ;[1 1 1] Attack 2
  (Utilities|FlowControl|DoOnce false :!label _label
    (:Completed
      (Utilities|FlowControl|Delay 0.1)
      (Animation|Montage|PlayMontage (Variables|Default|GetCharacterMesh) "/Game/Development/Animations/AnimationMontages/AM_SwordAttackShortLR.AM_SwordAttackShortLR"
        (:then
          (Variables|Default|SetAttackIndex 2)
          (goto _label Reset))))))

(event Custom|SwordAttack
  ;[0.051 0.051 0.051] SwordAttack
  (if (Variables|Default|GetisAttacking)
    (Variables|Default|SetsaveAttack true)
    (else
      (Variables|Default|SetIsAttacking true)
      (switch int (Variables|Default|GetAttackIndex)
        (:0
          (CallFunction|Attack1))
        (:1
          (CallFunction|Attack2))))))

(event Custom|RPC%20Attack1)

(event Custom|Attack3
  ;[1 1 1] Attack 3
  (Utilities|FlowControl|DoOnce false :!label _label
    (:Completed
      (Utilities|FlowControl|Delay 0.1)
      (Animation|Montage|PlayMontage (Variables|Default|GetCharacterMesh) "/Game/Development/Animations/AnimationMontages/AM_AttackSword2.AM_AttackSword2"
        (:then
          (Variables|Default|SetAttackIndex 3)
          (goto _label Reset))))))

(event Custom|Attack1
  ;[1 1 1] Attack 1
  (Utilities|FlowControl|DoOnce false :!label _label
    (:Completed
      (Utilities|FlowControl|Delay 0.1)
      (Animation|PlayAnimMontage (Game|GetPlayerCharacter 0) "/Game/Development/Animations/AnimationMontages/AM_AttackSwipRL.AM_AttackSwipRL" 1.0 "None")
      (Variables|Default|SetAttackIndex 1)
      (goto _label Reset))))

(event Custom|StopCombo
  ;[0.051 0.051 0.051] Stop Attack
  (Variables|Default|SetisAttacking false)
  (Variables|Default|SetAttackIndex 0))

(event Input|EnhancedActionEvents|EnhancedInputActionIA_BasicAttack
  (params (ActionValue :type Boolean) (ElapsedSeconds :type Float%20%28double-precision%29) (TriggeredSeconds :type Float%20%28double-precision%29) (InputAction :type Input%20Action%20Object%20Reference :default "/Game/ThirdPerson/Input/Actions/IA_BasicAttack.IA_BasicAttack"))
  ;[0.051 0.051 0.051] Attack Input
)

(event EventBeginPlay
  (bind _asbp_multiplayer_character (Utilities|Casting|CastToBP_MultiplayerCharacter (Components|GetOwner)))
  (Variables|Default|SetCharacterMesh (Variables|/Script/Engine.Character|GetMesh _asbp_multiplayer_character)))